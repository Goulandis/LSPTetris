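; BP_TetrisL is an L-shaped Tetris piece that adjusts its movement limits according to the direction it faces.
; The construction script backs up MoveLimitValue, and BeginPlay binds a handler to the EventTransformed event.
; AdjustMoveLimit lowers the UpMin bound by a fixed offset from its current value when facing left, and restores the backup for the other three orientations.
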(event `self.ReceiveBeginPlay`
  (`parent.ReceiveBeginPlay`)
  (add `self.EventTransformed` (`|CreateDelegate` :!event `AdjustMoveLimit`)))

(fn `AdjustMoveLimit`
  (bind (_movelimitvalue_upmin _movelimitvalue_upmax _movelimitvalue_movemin _movelimitvalue_movemax) (break `/Game/Datas/Struct/Stru_MoveLimit` (`self.MoveLimitValue`)))
  (switch `/Game/Datas/Enum/E_TetrisTowards` (`self.Towards`)
    (:`NewEnumerator0`
      (set `self.MoveLimitValue` (`self.MoveLimitValueBackup`) :!label _label))
    (:`NewEnumerator1`
      (set `self.MoveLimitValue` (make `/Game/Datas/Struct/Stru_MoveLimit` (- _movelimitvalue_upmin 100.0) _movelimitvalue_upmax _movelimitvalue_movemin _movelimitvalue_movemax)))
    (:`NewEnumerator2`
      (goto _label))
    (:`NewEnumerator3`
      (goto _label))))

(fn `UserConstructionScript`
  (`parent.UserConstructionScript`)
  (set `self.MoveLimitValueBackup` (`self.MoveLimitValue`)))