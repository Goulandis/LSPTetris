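; BP_TetrisN is a Tetris piece Blueprint, apparently the N shape, that adjusts its movement limits according to the direction it faces.
; The construction script caches the default MoveLimitValue, and BeginPlay binds a handler to the Transformed event.
; AdjustMoveLimit switches on Towards, lowering the current UpMin for Face Left and restoring the cached limits for the other three facings.
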(event `self.ReceiveBeginPlay`
  (`parent.ReceiveBeginPlay`)
  (add `self.EventTransformed` (`|CreateDelegate` :!event `AdjustMoveLimit`)))

(fn `AdjustMoveLimit`
  (bind (_movelimitvalue_upmin _movelimitvalue_upmax _movelimitvalue_movemin _movelimitvalue_movemax) (break `/Game/Datas/Struct/Stru_MoveLimit` (`self.MoveLimitValue`)))
  (switch `/Game/Datas/Enum/E_TetrisTowards` (`self.Towards`)
    (:`NewEnumerator0`
      (set `self.MoveLimitValue` (`self.MoveLimitValueBackup`) :!label _label))
    (:`NewEnumerator1`
      (set `self.MoveLimitValue` (make `/Game/Datas/Struct/Stru_MoveLimit` (- _movelimitvalue_upmin 100.0) _movelimitvalue_upmax _movelimitvalue_movemin _movelimitvalue_movemax)))
    (:`NewEnumerator2`
      (goto _label))
    (:`NewEnumerator3`
      (goto _label))))

(fn `UserConstructionScript`
  (`parent.UserConstructionScript`)
  (set `self.MoveLimitValueBackup` (`self.MoveLimitValue`)))