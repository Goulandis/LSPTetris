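; Base actor for a player-controlled Tetris piece that falls in timed steps and takes move, rotate and hasten input.
; A per-piece BP_TetrisConfig object holds speeds and permission flags, which MoveLimit updates at side and floor bounds.
; Moves and rotations fire events, with rotation also deriving orientation from an arrow's forward vector.
; Hasten locks other actions while Tick drops the piece to the floor, where Falled disables input.
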(event `self.ReceiveBeginPlay`
  (`self.EnableInput` (`GameplayStatics.GetPlayerController` 0))
  (`KismetSystemLibrary.K2_SetTimerDelegate` (delegate `Falling`) (`/Game/Blueprints/Obj/BP_TetrisConfig.FallInterval` (`self.ConfigObj`)) true)
  (add `self.EventMoved` (`|CreateDelegate` :!event `MoveLimit`))
  (add `self.EventFalled` (`|CreateDelegate` :!event `Falled`)))

(event `self.ReceiveTick`
  (params (DeltaSeconds :type "Float (single-precision)"))
  (bind (_returnvalue_x _returnvalue_y) (`KismetMathLibrary.BreakVector` (`self.K2_GetActorLocation`)))
  (bind (_returnvalue_x_2 _returnvalue_y_2 _returnvalue_z) (`KismetMathLibrary.BreakVector` (`self.K2_GetActorLocation`)))
  (bind (_returnvalue_x_3 _returnvalue_y_3 _returnvalue_z_2) (`KismetMathLibrary.BreakVector` (`self.K2_GetActorLocation`)))
  (bind _movelimitvalue_upmin (break `/Game/Datas/Struct/Stru_MoveLimit` (`self.MoveLimitValue`)))
  (bind _movelimitvalue_upmin_2 (break `/Game/Datas/Struct/Stru_MoveLimit` (`self.MoveLimitValue`)))
  (bind (_iscanmove_iscanleft _iscanmove_iscanright _iscanmove_iscandown _iscanmove_iscantransform _iscanmove_iscanhastenfall) (break `/Game/Datas/Struct/Stru_IsCanControl` (`/Game/Blueprints/Obj/BP_TetrisConfig.IsCanMove` (`self.ConfigObj`))))
  (if _iscanmove_iscanhastenfall
    (`self.K2_SetActorLocation` (`KismetMathLibrary.MakeVector` _returnvalue_x_2 _returnvalue_y_2 (- _returnvalue_z (`/Game/Blueprints/Obj/BP_TetrisConfig.FallHasten` (`self.ConfigObj`)))))
    (if (<= _returnvalue_z_2 _movelimitvalue_upmin_2)
      (`self.Falled`)
      (`self.K2_SetActorLocation` (`KismetMathLibrary.MakeVector` _returnvalue_x _returnvalue_y _movelimitvalue_upmin)))))

(event `Falling`
  (bind (_returnvalue_x _returnvalue_y _returnvalue_z) (`KismetMathLibrary.BreakVector` (`self.K2_GetActorLocation`)))
  (bind (_iscanmove_iscanleft _iscanmove_iscanright _iscanmove_iscandown) (break `/Game/Datas/Struct/Stru_IsCanControl` (`/Game/Blueprints/Obj/BP_TetrisConfig.IsCanMove` (`self.ConfigObj`))))
  (if _iscanmove_iscandown
    (`self.K2_SetActorLocation` (`KismetMathLibrary.MakeVector` _returnvalue_x _returnvalue_y (- _returnvalue_z (`/Game/Blueprints/Obj/BP_TetrisConfig.FallSpeed` (`self.ConfigObj`)))))
    (`self.EventMoved` (`self.K2_GetActorLocation`))))

(event `InputAction|Transform`
  (params (Key :type "Key Structure"))
  (bind (_returnvalue_roll _returnvalue_pitch _returnvalue_yaw) (`KismetMathLibrary.BreakRotator` (`self.K2_GetActorRotation`)))
  (bind (_iscanmove_iscanleft _iscanmove_iscanright _iscanmove_iscandown _iscanmove_iscantransform) (break `/Game/Datas/Struct/Stru_IsCanControl` (`/Game/Blueprints/Obj/BP_TetrisConfig.IsCanMove` (`self.ConfigObj`))))
  (:`Pressed`
    (if (and _iscanmove_iscandown _iscanmove_iscantransform)
      (`self.K2_SetActorRotation` (`KismetMathLibrary.MakeRotator` (+ _returnvalue_roll (`/Game/Blueprints/Obj/BP_TetrisConfig.RotationAmount` (`self.ConfigObj`))) _returnvalue_pitch _returnvalue_yaw))
      (`self.UpdateTowards`)
      (`self.EventTransformed`))))

(event `InputAction|MoveRight`
  (params (Key :type "Key Structure"))
  (bind (_returnvalue_x _returnvalue_y _returnvalue_z) (`KismetMathLibrary.BreakVector` (`self.K2_GetActorLocation`)))
  (bind (_iscanmove_iscanleft _iscanmove_iscanright _iscanmove_iscandown) (break `/Game/Datas/Struct/Stru_IsCanControl` (`/Game/Blueprints/Obj/BP_TetrisConfig.IsCanMove` (`self.ConfigObj`))))
  (:`Pressed`
    (if (and _iscanmove_iscanright _iscanmove_iscandown)
      (`self.K2_SetActorLocation` (`KismetMathLibrary.MakeVector` _returnvalue_x (+ _returnvalue_y (`/Game/Blueprints/Obj/BP_TetrisConfig.MoveSpeed` (`self.ConfigObj`))) _returnvalue_z))
      (`self.EventMoved` (`self.K2_GetActorLocation`)))))

(event `InputAction|MoveLeft`
  (params (Key :type "Key Structure"))
  (bind (_returnvalue_x _returnvalue_y _returnvalue_z) (`KismetMathLibrary.BreakVector` (`self.K2_GetActorLocation`)))
  (bind (_iscanmove_iscanleft _iscanmove_iscanright _iscanmove_iscandown) (break `/Game/Datas/Struct/Stru_IsCanControl` (`/Game/Blueprints/Obj/BP_TetrisConfig.IsCanMove` (`self.ConfigObj`))))
  (:`Pressed`
    (if (and _iscanmove_iscanleft _iscanmove_iscandown)
      (`self.K2_SetActorLocation` (`KismetMathLibrary.MakeVector` _returnvalue_x (- _returnvalue_y (`/Game/Blueprints/Obj/BP_TetrisConfig.MoveSpeed` (`self.ConfigObj`))) _returnvalue_z))
      (`self.EventMoved` (`self.K2_GetActorLocation`)))))

(event `InputAction|Hasten`
  (params (Key :type "Key Structure"))
  (bind _configobj (`self.ConfigObj`))
  (bind (_iscanmove_iscanleft _iscanmove_iscanright _iscanmove_iscandown _iscanmove_iscantransform _iscanmove_iscanhastenfall) (break `/Game/Datas/Struct/Stru_IsCanControl` (`/Game/Blueprints/Obj/BP_TetrisConfig.IsCanMove` _configobj)))
  (:`Pressed`
    (if (and _iscanmove_iscandown _iscanmove_iscanhastenfall)
      (set `/Game/Blueprints/Obj/BP_TetrisConfig.IsCanMove` (make `/Game/Datas/Struct/Stru_IsCanControl` false false false false true) _configobj))))

(fn `Falled`
  (set `/Game/Blueprints/Obj/BP_TetrisConfig.IsCanMove` (make `/Game/Datas/Struct/Stru_IsCanControl` false) (`self.ConfigObj`))
  (`self.DisableInput` (`GameplayStatics.GetPlayerController` 0)))

(fn `MoveLimit`
  (params (CPos :type "Vector Structure"))
  (locals (IsCanLeft :type Boolean :default true) (IsCanRight :type Boolean :default true) (IsCanDwon :type Boolean :default true) (IsCanTransform :type Boolean :default true) (IsCanHastenFall :type Boolean :default true))
  (bind (_movelimitvalue_upmin _movelimitvalue_upmax _movelimitvalue_movemin _movelimitvalue_movemax) (break `/Game/Datas/Struct/Stru_MoveLimit` (`self.MoveLimitValue`)))
  (bind (_iscanmove_iscanleft _iscanmove_iscanright _iscanmove_iscandown) (break `/Game/Datas/Struct/Stru_IsCanControl` (`/Game/Blueprints/Obj/BP_TetrisConfig.IsCanMove` (`self.ConfigObj`))))
  (if _iscanmove_iscandown
    (`|ExecutionSequence`
      (:`then_0`
        (if (<= CPos_Y _movelimitvalue_movemin)
          (set `local.IsCanLeft` false)))
      (:`then_1`
        (if (>= CPos_Y _movelimitvalue_movemax)
          (set `local.IsCanRight` false)))
      (:`then_2`
        (if (<= CPos_Z _movelimitvalue_upmin)
          (set `local.IsCanDwon` false)
          (`self.EventFalled`)))
      (:`then_3`
        (set `/Game/Blueprints/Obj/BP_TetrisConfig.IsCanMove` (make `/Game/Datas/Struct/Stru_IsCanControl` (`local.IsCanLeft`) (`local.IsCanRight`) (`local.IsCanDwon`) (`local.IsCanTransform`) (`local.IsCanHastenFall`)) (`self.ConfigObj`))))))

(fn `UpdateTowards`
  (locals (FaceUp :type "Vector Structure" :default (0.0 0.0 1.0)) (FaceLeft :type "Vector Structure" :default (0.0 -1.0 0.0)) (FaceDown :type "Vector Structure" :default (0.0 0.0 -1.0)) (FaceRight :type "Vector Structure" :default (0.0 1.0 0.0)) (Offset :type "Float (double-precision)" :default 0.5))
  (bind _offset (`local.Offset`))
  (bind _returnvalue (`SceneComponent.GetForwardVector` (`self.Arrow`)))
  (`|ExecutionSequence`
    (:`then_0`
      (if (== _returnvalue (`local.FaceUp`) :`ErrorTolerance` _offset)
        (set `self.Towards` "NewEnumerator0")
        (else
          (`/Game/Blueprints/FunLib/DebugFunLib.DebugLog` "Error:UpdateTowards" "The current orientation is not defined" :!label _label))))
    (:`then_1`
      (if (== _returnvalue (`local.FaceLeft`) :`ErrorTolerance` _offset)
        (set `self.Towards` "NewEnumerator1")
        (else
          (goto _label))))
    (:`then_2`
      (if (== _returnvalue (`local.FaceDown`) :`ErrorTolerance` _offset)
        (set `self.Towards` "NewEnumerator2")
        (else
          (goto _label))))
    (:`then_3`
      (if (== _returnvalue (`local.FaceRight`) :`ErrorTolerance` _offset)
        (set `self.Towards` "NewEnumerator3")
        (else
          (goto _label))))))

(fn `UserConstructionScript`
  (bind _returnvalue (`|GenericCreateObject` "/Game/Blueprints/Obj/BP_TetrisConfig.BP_TetrisConfig_C"))
  (set `self.ConfigObj` _returnvalue)
  (`self.K2_SetActorLocation` (`self.ConstructPos`)))